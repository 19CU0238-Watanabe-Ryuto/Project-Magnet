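; OnewayWall is a barrier actor that starts passable and turns solid once enough players and the ball have passed through it.
; End-overlap events on the wall count ThirdPersonCharacters and flag the AttractObject_Ball, without checking direction.
; When both conditions hold, Tick switches collision to block once and ramps a custom primitive data float over OpacityTime to drive the material's opacity.
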(event OnComponentEndOverlap(Wall)
  (params (OverlappedComponent :type Primitive%20Component%20Object%20Reference) (OtherActor :type Actor%20Object%20Reference) (OtherComp :type Primitive%20Component%20Object%20Reference) (OtherBodyIndex :type Integer))
  (Utilities|Casting|CastToThirdPersonCharacter OtherActor
    (:then
      (Math|Integer|IncrementInt (Variables|Default|GetplayerCount)))
    (:CastFailed
      (Utilities|Casting|CastToAttractObject_Ball OtherActor)
      (Variables|Default|SetballOverlap true))))

(event EventBeginPlay
  (Collision|SetCollisionProfileName (Variables|Default|GetWall) "OverlapAllDynamic" true :!class /Script/Engine.PrimitiveComponent)
  (Rendering|Material|SetMaterial (Variables|Default|GetWall) 0 "/Game/Effect/InvisibleWall/OnewayWall_Mat.OnewayWall_Mat"))

(event EventTick
  (params (DeltaSeconds :type Float%20%28single-precision%29))
  (Variables|Default|SetDelta%20Seconds DeltaSeconds)
  (if (and (>= (Variables|Default|GetplayerCount) (Variables|Default|GetplayerNum)) (Variables|Default|GetballOverlap))
    (Utilities|SetOpacityMacro)
    (Utilities|FlowControl|DoOnce false
      (:Completed
        (Collision|SetCollisionProfileName (Variables|Default|GetWall) "BlockAllDynamic" true :!class /Script/Engine.PrimitiveComponent)))))

(fn ConstructionScript)