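; Procedural modular building actor that assembles its four facades from tiled static meshes in the Construction Script.
; Per-face loops over floor and tile counts pick bottom, wall and top pieces, with pillars at front and back corners.
; Flags add a front door and stairs or make either side windowless.
; Each piece goes through CreateMesh, which adds a component and sets mesh and material slots, using negative scale for mirroring.
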(event EventBeginPlay)

(event Collision|EventActorBeginOverlap
  (params (OtherActor :type Actor%20Object%20Reference)))

(event EventTick
  (params (DeltaSeconds :type Float%20%28single-precision%29)))

(fn ConstructionScript
  (bind _pillars (Variables|Default|GetPillars))
  (bind _floor_amount (Variables|Default|GetFloor_Amount))
  (bind _floor_amount_2 (Variables|Default|GetFloor_Amount))
  (bind _floor_amount_3 (Variables|Default|GetFloor_Amount))
  (bind _floor_amount_4 (Variables|Default|GetFloor_Amount))
  (bind _pillartop (Variables|Default|GetPillarTop))
  (bind _door_position (Variables|Default|GetDoor_Position))
  (bind _pillars_2 (Variables|Default|GetPillars))
  (bind _pillartop_2 (Variables|Default|GetPillarTop))
  (bind _returnvalue (- _floor_amount 1))
  (bind _returnvalue_2 (- _floor_amount_2 1))
  (bind _returnvalue_3 (- _floor_amount_4 1))
  (bind _returnvalue_4 (- _floor_amount_3 1))
  ;[1 1 1] 建物の４面とも同じシーケンスで管理
  (Utilities|FlowControl|Sequence
    (:then_0
      ;[1 0.9294 0.4354] 正面
      ;;[1 1 1] 縦の繰り返し
      ;;;[1 1 1] 繰り返し
      (for _index (range 0 _returnvalue_3)
        (Utilities|FlowControl|Sequence
          (:then_0
            (if (< _index _returnvalue_3)
              ;;[0.3544 1 0.008445] 端のメッシュ
              (CallFunction|CreateMesh (Math|Transform|MakeTransform (Math|Vector|MakeVector (* (- (Variables|Default|GetX%20Amount) 1) (Variables|Default|GetX%20Tile)) 0.0 (* _index (Variables|Default|GetZ%20Tile)))) _pillars)
              (CallFunction|CreateMesh (Math|Transform|MakeTransform (Math|Vector|MakeVector (* -1 (Variables|Default|GetX%20Tile)) 0.0 (* _index (Variables|Default|GetZ%20Tile))) "0, 0, 0" "-1.000000,1,1") _pillars)
              (else
                (CallFunction|CreateMesh (Math|Transform|MakeTransform (Math|Vector|MakeVector (* (- (Variables|Default|GetX%20Amount) 1) (Variables|Default|GetX%20Tile)) 0.0 (* _index (Variables|Default|GetZ%20Tile)))) _pillartop)
                (CallFunction|CreateMesh (Math|Transform|MakeTransform (Math|Vector|MakeVector (* -1 (Variables|Default|GetX%20Tile)) 0.0 (* _index (Variables|Default|GetZ%20Tile))) "0, 0, 0" "-1.000000,1,1") _pillartop))))
          (:then_1
            ;;[1 1 1] 横の繰り返し
            (for _index_2 (range 0 (- (Variables|Default|GetX%20Amount) 1))
              (Utilities|FlowControl|Sequence
                (:then_0
                  (if (== _index _returnvalue_3)
                    ;;[0.8691 1 0.272] 天辺のメッシュ
                    ;;;[1 1 1] メッシュ生成
                    (CallFunction|CreateMesh (Math|Transform|MakeTransform (Math|Vector|MakeVector (* _index_2 (Variables|Default|GetX%20Tile)) 0.0 (* _index (Variables|Default|GetZ%20Tile)))) (Variables|Default|GetTopMesh))
                    (elif (Variables|Default|GetHasDoor)
                      ;;[0.7809 1 0.3217] 入口のメッシュ
                      (if (== _index 0)
                        (if (== _index_2 (- _door_position 1))
                          ;;;[1 1 1] 扉のメッシュを生成
                          (CallFunction|CreateMesh (Math|Transform|MakeTransform (Math|Vector|MakeVector (* _index_2 (Variables|Default|GetX%20Tile)) 0.0 (* _index (Variables|Default|GetZ%20Tile)))) (Variables|Default|GetDoor))
                          (elif (not (== (- _door_position 2) _index_2))
                            ;;;[1 1 1] 扉がない位置には、別のメッシュを生成する
                            (CallFunction|CreateMesh (Math|Transform|MakeTransform (Math|Vector|MakeVector (* _index_2 (Variables|Default|GetX%20Tile)) 0.0 (* _index (Variables|Default|GetZ%20Tile)))) (Variables|Default|GetBottomMesh) :!label _label)))
                        (else
                          ;;[0.6902 1 0.1808] ベースのメッシュ
                          ;;;[1 1 1] メッシュ生成
                          (CallFunction|CreateMesh (Math|Transform|MakeTransform (Math|Vector|MakeVector (* _index_2 (Variables|Default|GetX%20Tile)) 0.0 (* _index (Variables|Default|GetZ%20Tile)))) (Variables|Default|GetWall))))
                      (else
                        (goto _label)))))
                (:then_1
                  (if (Variables|Default|GetHasStairs)
                    ;;[0.2603 0.3333 0.1072] 階段のメッシュ
                    ;;;[1 1 1] 階段
                    (if (and (> _index (Variables|Default|GetStair_Amount)) (< _index (- (Variables|Default|GetFloor_Amount) 1)))
                      (if (== _index_2 (- (Variables|Default|GetStairPosition) 1))
                        (if (>= (Variables|Default|GetFloor_Amount) 5)
                          ;;;;[1 1 1] 階段のメッシュを生成
                          (CallFunction|CreateMesh (Math|Transform|MakeTransform (Math|Vector|MakeVector (* _index_2 (Variables|Default|GetX%20Tile)) 0.0 (* _index (Variables|Default|GetZ%20Tile)))) (Variables|Default|GetStairMesh)))))))))))))
    (:then_1
      ;[1 0.5426 0.9995] 左面
      ;;[1 1 1] 縦の繰り返し
      ;;;[1 1 1] 繰り返し
      (for _index_3 (range 0 _returnvalue_2)
        ;;[1 1 1] 奥の繰り返し
        (for _index_4 (range 0 (- (Variables|Default|GetY%20Amout) 1))
          (Utilities|FlowControl|Sequence
            (:then_0
              (if (== _index_3 _returnvalue_2)
                (if (Variables|Default|GetHasNoWindowLeft)
                  ;;[0.8691 1 0.272] 天辺のメッシュ
                  ;;;[1 1 1] メッシュ生成
                  (CallFunction|CreateMesh (Math|Transform|MakeTransform (Math|Vector|MakeVector (+ (* (- (Variables|Default|GetX%20Amount) 1) (Variables|Default|GetX%20Tile)) 135.0) (+ (* (Math|Float|Truncate (* _index_4 -1.0)) (Variables|Default|GetX%20Tile)) -1e+02) (* _index_3 (Variables|Default|GetZ%20Tile))) "0,90.000000, 0" "1.000000,-1.000000,1") (Variables|Default|GetNoWindowTop))
                  (else
                    ;;;[1 1 1] メッシュ生成
                    (CallFunction|CreateMesh (Math|Transform|MakeTransform (Math|Vector|MakeVector (+ (* (- (Variables|Default|GetX%20Amount) 1) (Variables|Default|GetX%20Tile)) 135.0) (+ (* (Math|Float|Truncate (* _index_4 -1.0)) (Variables|Default|GetX%20Tile)) -1e+02) (* _index_3 (Variables|Default|GetZ%20Tile))) "0,90.000000, 0" "1.000000,-1.000000,1") (Variables|Default|GetTopMesh))))
                (elif (Variables|Default|GetHasNoWindowLeft)
                  ;;[0.7809 1 0.3217] 1階のメッシュ
                  (CallFunction|CreateMesh (Math|Transform|MakeTransform (Math|Vector|MakeVector (+ (* (- (Variables|Default|GetX%20Amount) 1) (Variables|Default|GetX%20Tile)) 135.0) (+ (* (Math|Float|Truncate (* _index_4 -1.0)) (Variables|Default|GetX%20Tile)) -1e+02) (* _index_3 (Variables|Default|GetZ%20Tile))) "0,90.000000,0.000000" "1.000000,-1.000000,1.000000") (Variables|Default|GetNoWindow))
                  (elif (== _index_3 0)
                    ;;;[1 1 1] 扉がない位置には、別のメッシュを生成する
                    (CallFunction|CreateMesh (Math|Transform|MakeTransform (Math|Vector|MakeVector (+ (* (- (Variables|Default|GetX%20Amount) 1) (Variables|Default|GetX%20Tile)) 135.0) (+ (* (Math|Float|Truncate (* _index_4 -1.0)) (Variables|Default|GetX%20Tile)) -1e+02) (* _index_3 (Variables|Default|GetZ%20Tile))) "0,90.000000,0.000000" "1.000000,-1.000000,1.000000") (Variables|Default|GetBottomMesh))))))
            (:then_1
              ;;[0.6902 1 0.1808] ベースのメッシュ
              (if (not (>= _index_3 _returnvalue_2))
                (if (Variables|Default|GetHasNoWindowLeft)
                  ;;;[1 1 1] メッシュ生成
                  (CallFunction|CreateMesh (Math|Transform|MakeTransform (Math|Vector|MakeVector (+ (* (- (Variables|Default|GetX%20Amount) 1) (Variables|Default|GetX%20Tile)) 135.0) (+ (* (Math|Float|Truncate (* _index_4 -1.0)) (Variables|Default|GetX%20Tile)) -1e+02) (* _index_3 (Variables|Default|GetZ%20Tile))) "0,90.000000,0.000000" "1.000000,-1.000000,1.000000") (Variables|Default|GetNoWindow))
                  (else
                    ;;;[1 1 1] メッシュ生成
                    (CallFunction|CreateMesh (Math|Transform|MakeTransform (Math|Vector|MakeVector (+ (* (- (Variables|Default|GetX%20Amount) 1) (Variables|Default|GetX%20Tile)) 135.0) (+ (* (Math|Float|Truncate (* _index_4 -1.0)) (Variables|Default|GetX%20Tile)) -1e+02) (* _index_3 (Variables|Default|GetZ%20Tile))) "0,90.000000,0.000000" "1.000000,-1.000000,1.000000") (Variables|Default|GetWall))))))))))
    (:then_2
      ;[1 0.3512 0.4109] 右面
      ;;[1 1 1] 縦の繰り返し
      ;;;[1 1 1] 繰り返し
      (for _index_5 (range 0 _returnvalue)
        ;;[1 1 1] 奥の繰り返し
        (for _index_6 (range 0 (- (Variables|Default|GetY%20Amout) 1))
          (Utilities|FlowControl|Sequence
            (:then_0
              (if (== _index_5 _returnvalue)
                (if (Variables|Default|GetHasNoWindowRight)
                  ;;[0.8691 1 0.272] 天辺のメッシュ
                  ;;;[1 1 1] メッシュ生成(窓なし）
                  (CallFunction|CreateMesh (Math|Transform|MakeTransform (Math|Vector|MakeVector (+ (* (- 0 1) (Variables|Default|GetX%20Tile)) -135.0) (+ (* (Math|Float|Truncate (* _index_6 -1.0)) (Variables|Default|GetX%20Tile)) -1e+02) (* _index_5 (Variables|Default|GetZ%20Tile))) "0,90.000000, 0") (Variables|Default|GetNoWindowTop))
                  (else
                    ;;;[1 1 1] メッシュ生成（窓あり）
                    (CallFunction|CreateMesh (Math|Transform|MakeTransform (Math|Vector|MakeVector (+ (* (- 0 1) (Variables|Default|GetX%20Tile)) -135.0) (+ (* (Math|Float|Truncate (* _index_6 -1.0)) (Variables|Default|GetX%20Tile)) -1e+02) (* _index_5 (Variables|Default|GetZ%20Tile))) "0,90.000000, 0") (Variables|Default|GetTopMesh))))
                (elif (Variables|Default|GetHasNoWindowRight)
                  ;;[0.7809 1 0.3217] 1階のメッシュ
                  ;;;[1 1 1] 扉がない位置には、別のメッシュを生成する（窓なし）
                  (CallFunction|CreateMesh (Math|Transform|MakeTransform (Math|Vector|MakeVector (+ (* (- 0 1) (Variables|Default|GetX%20Tile)) -135.0) (+ (* (Math|Float|Truncate (* _index_6 -1.0)) (Variables|Default|GetX%20Tile)) -1e+02) (* _index_5 (Variables|Default|GetZ%20Tile))) "0,90.000000,0.000000") (Variables|Default|GetNoWindow))
                  (elif (== _index_5 0)
                    ;;;[1 1 1] 扉がない位置には、別のメッシュを生成する
                    (CallFunction|CreateMesh (Math|Transform|MakeTransform (Math|Vector|MakeVector (+ (* (- 0 1) (Variables|Default|GetX%20Tile)) -135.0) (+ (* (Math|Float|Truncate (* _index_6 -1.0)) (Variables|Default|GetX%20Tile)) -1e+02) (* _index_5 (Variables|Default|GetZ%20Tile))) "0,90.000000,0.000000") (Variables|Default|GetBottomMesh))))))
            (:then_1
              ;;[0.6902 1 0.1808] ベースのメッシュ
              (if (not (>= _index_5 _returnvalue))
                (if (Variables|Default|GetHasNoWindowRight)
                  ;;;[1 1 1] メッシュ生成
                  (CallFunction|CreateMesh (Math|Transform|MakeTransform (Math|Vector|MakeVector (+ (* (- 0 1) (Variables|Default|GetX%20Tile)) -135.0) (+ (* (Math|Float|Truncate (* _index_6 -1.0)) (Variables|Default|GetX%20Tile)) -1e+02) (* _index_5 (Variables|Default|GetZ%20Tile))) "0,90.000000,0.000000") (Variables|Default|GetNoWindow))
                  (else
                    ;;;[1 1 1] メッシュ生成
                    (CallFunction|CreateMesh (Math|Transform|MakeTransform (Math|Vector|MakeVector (+ (* (- 0 1) (Variables|Default|GetX%20Tile)) -135.0) (+ (* (Math|Float|Truncate (* _index_6 -1.0)) (Variables|Default|GetX%20Tile)) -1e+02) (* _index_5 (Variables|Default|GetZ%20Tile))) "0,90.000000,0.000000") (Variables|Default|GetWall))))))))))
    (:then_3
      ;[1 0.9294 0.4354] 後ろ面
      ;;[1 1 1] 縦の繰り返し
      ;;;[1 1 1] 繰り返し
      (for _index_7 (range 0 _returnvalue_4)
        ;;[1 1 1] 横の繰り返し
        (Utilities|FlowControl|Sequence
          (:then_0
            ;;[0.3544 1 0.008445] 端のメッシュ
            (if (< _index_7 _returnvalue_4)
              (CallFunction|CreateMesh (Math|Transform|MakeTransform (Math|Vector|MakeVector (* (- (Variables|Default|GetX%20Amount) 1) (Variables|Default|GetX%20Tile)) (+ (* (Math|Float|Truncate (* (Variables|Default|GetY%20Amout) -1.0)) (Variables|Default|GetX%20Tile)) -2e+02) (* _index_7 (Variables|Default|GetZ%20Tile))) "0, 0, 0" "1,-1.000000,1") _pillars_2)
              (CallFunction|CreateMesh (Math|Transform|MakeTransform (Math|Vector|MakeVector (* -1 (Variables|Default|GetX%20Tile)) (+ (* (Math|Float|Truncate (* (Variables|Default|GetY%20Amout) -1.0)) (Variables|Default|GetX%20Tile)) -2e+02) (* _index_7 (Variables|Default|GetZ%20Tile))) "0, 0, 0" "-1.000000,-1.000000,1") _pillars_2)
              (else
                (CallFunction|CreateMesh (Math|Transform|MakeTransform (Math|Vector|MakeVector (* (- (Variables|Default|GetX%20Amount) 1) (Variables|Default|GetX%20Tile)) (+ (* (Math|Float|Truncate (* (Variables|Default|GetY%20Amout) -1.0)) (Variables|Default|GetX%20Tile)) -2e+02) (* _index_7 (Variables|Default|GetZ%20Tile))) "0, 0, 0" "1,-1.000000,1") _pillartop_2)
                (CallFunction|CreateMesh (Math|Transform|MakeTransform (Math|Vector|MakeVector (* -1 (Variables|Default|GetX%20Tile)) (+ (* (Math|Float|Truncate (* (Variables|Default|GetY%20Amout) -1.0)) (Variables|Default|GetX%20Tile)) -2e+02) (* _index_7 (Variables|Default|GetZ%20Tile))) "0, 0, 0" "-1.000000,-1.000000,1") _pillartop_2))))
          (:then_1
            (for _index_8 (range 0 (- (Variables|Default|GetX%20Amount) 1))
              (Utilities|FlowControl|Sequence
                (:then_0
                  (if (== _index_7 _returnvalue_4)
                    ;;[0.8691 1 0.272] 天辺のメッシュ
                    ;;;[1 1 1] メッシュ生成
                    (CallFunction|CreateMesh (Math|Transform|MakeTransform (Math|Vector|MakeVector (* _index_8 (Variables|Default|GetX%20Tile)) (+ (* (Math|Float|Truncate (* (Variables|Default|GetY%20Amout) -1.0)) (Variables|Default|GetX%20Tile)) -2e+02) (* _index_7 (Variables|Default|GetZ%20Tile))) "0, 0, 0" "1,-1.000000,1") (Variables|Default|GetTopMesh))
                    (else
                      ;;[0.7809 1 0.3217] 入口のメッシュ
                      (if (== _index_7 0)
                        ;;;[1 1 1] 扉がない位置には、別のメッシュを生成する
                        (CallFunction|CreateMesh (Math|Transform|MakeTransform (Math|Vector|MakeVector (* _index_8 (Variables|Default|GetX%20Tile)) (+ (* (Math|Float|Truncate (* (Variables|Default|GetY%20Amout) -1.0)) (Variables|Default|GetX%20Tile)) -2e+02) (* _index_7 (Variables|Default|GetZ%20Tile))) "0, 0, 0" "1,-1.000000,1.000000") (Variables|Default|GetBottomMesh))
                        (else
                          ;;[0.6902 1 0.1808] ベースのメッシュ
                          ;;;[1 1 1] メッシュ生成
                          (CallFunction|CreateMesh (Math|Transform|MakeTransform (Math|Vector|MakeVector (* _index_8 (Variables|Default|GetX%20Tile)) (+ (* (Math|Float|Truncate (* (Variables|Default|GetY%20Amout) -1.0)) (Variables|Default|GetX%20Tile)) -2e+02) (* _index_7 (Variables|Default|GetZ%20Tile))) "0, 0, 0" "1,-1.000000,1.000000") (Variables|Default|GetWall)))))))))))))))

(fn CreateMesh
  (params (Transform :type Transform) (Mesh :type Static%20Mesh%20Object%20Reference))
  ;[1 1 1] メッシュを生成
  (bind _returnvalue (AddComponent|AddStaticMeshComponent false Transform))
  ;[1 1 1] メッシュをセットする
  (Components|StaticMesh|SetStaticMesh _returnvalue Mesh)
  ;[1 1 1] セットされたメッシュにマテリアルを追加
  (Rendering|Material|SetMaterial _returnvalue 0 0)
  (Rendering|Material|SetMaterial _returnvalue 1 0))