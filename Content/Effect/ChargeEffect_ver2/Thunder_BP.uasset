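; Thunder effect actor in the charge effect set that makes lightning beams flicker around it.
; Every Tick it gives the Thunder1 and Thunder2 beam components new random end points and start tangents through their vector variables, biased to non-negative Z.
; Matching update chains for Thunder3 through Thunder7 exist but are disconnected and never run.
; BeginPlay, overlap and the construction script are empty.
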(event EventBeginPlay)

(event Collision|EventActorBeginOverlap
  (params (OtherActor :type Actor%20Object%20Reference)))

(event EventTick
  (params (DeltaSeconds :type Float%20%28single-precision%29))
  (bind _thunder2 (Variables|Default|GetThunder2))
  (bind _thunder1 (Variables|Default|GetThunder1))
  (Niagara|SetNiagaraVariable(Vector3) _thunder1 "Beam End" (Math|Vector|MakeVector (Math|Random|RandomFloatinRange -1e+02 1e+02) (Math|Random|RandomFloatinRange -1e+02 1e+02) (Math|Random|RandomFloatinRange 0.0 1e+02)))
  (Niagara|SetNiagaraVariable(Vector3) _thunder1 "Vector_Beam Start Tangent" (Math|Vector|MakeVector (Math|Random|RandomFloatinRange -5.0 5.0) (Math|Random|RandomFloatinRange -5.0 5.0) (Math|Random|RandomFloatinRange 0.0 5.0)))
  (Niagara|SetNiagaraVariable(Vector3) _thunder2 "Beam End" (Math|Vector|MakeVector (Math|Random|RandomFloatinRange -1e+02 1e+02) (Math|Random|RandomFloatinRange -1e+02 1e+02) (Math|Random|RandomFloatinRange 0.0 1e+02)))
  (Niagara|SetNiagaraVariable(Vector3) _thunder2 "Vector_Beam Start Tangent" (Math|Vector|MakeVector (Math|Random|RandomFloatinRange -5.0 5.0) (Math|Random|RandomFloatinRange -5.0 5.0) (Math|Random|RandomFloatinRange 0.0 5.0))))

(fn ConstructionScript)