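; Team goal for a magnet ball game that scores balls carried or shot in by players.
; Overlaps on GoalCollision-tagged components award touchdown or shot points through MagnetGameInstance, or require HaveTrophy when CanOwnGoal is set, then hand the ball to the goal.
; After ShootTime, Tick launches the ball back out with random power along a randomly rotated arrow, whose length reflects that power.
; Goal color is passed to the mesh as custom primitive data.
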(event OnComponentBeginOverlap(Collision)
  (params (OverlappedComponent :type Primitive%20Component%20Object%20Reference) (OtherActor :type Actor%20Object%20Reference) (OtherComp :type Primitive%20Component%20Object%20Reference) (OtherBodyIndex :type Integer) (bFromSweep :type Boolean) (SweepResult :type Hit%20Result%20Structure%20%28by%20ref%29))
  (if (Components|ComponentHasTag OtherComp "GoalCollision")
    (Variables|Default|SethitActor OtherActor)
    (bind _asmagnet_game_instance (Utilities|Casting|CastToMagnetGameInstance (Game|GetGameInstance)))
    (Variables|Default|SetcastedMagnetGameInstance _asmagnet_game_instance)
    (if (Variables|Default|GetcanOwnGoal)
      (Variables|Default|SetplayerMatch false)
      (bind _array_index (Utilities|Array|ForEachLoopwithBreak (Variables|/Game/Blueprints/MagnetGameInstance.MagnetGameInstance_C|GetPlayerActorArray (Variables|Default|GetcastedMagnetGameInstance)) :!label _label)
        (:LoopBody
          (if (== (Variables|Default|GethitActor) (Game|Player|GetPlayerPawn _array_index))
            (Variables|Default|SetplayerMatch true)
            (goto _label Break)))
        (:Completed
          (if (Variables|Default|GetplayerMatch)
            (bind _asthird_person_character (Utilities|Casting|CastToThirdPersonCharacter (Variables|Default|GethitActor)))
            (bind _output_get (Variables|Default|SetcastedPlayerActor _asthird_person_character))
            (if (Variables|/Game/ThirdPersonBP/Blueprints/ThirdPersonCharacter.ThirdPersonCharacter_C|GethaveTrophy _output_get)
              (if (not (Variables|Default|GetisGoal)) :!label _label_2
                (Variables|Default|SetisGoal true)
                ;[1 1 1] ゲームが制限時間以内かチェック
                (bind _asmagnet_game_instance_2 (Utilities|Casting|CastToMagnetGameInstance (Game|GetGameInstance)))
                (bind _output_get_2 (Variables|Default|SetcastedMagnetGameInstance _asmagnet_game_instance_2))
                (if (not (Variables|/Game/Blueprints/MagnetGameInstance.MagnetGameInstance_C|GetisGameSet _output_get_2))
                  (Variables|/Game/ThirdPersonBP/Blueprints/ThirdPersonCharacter.ThirdPersonCharacter_C|SethaveTrophy (Variables|Default|GetcastedPlayerActor) false)
                  (Default|SetScore (Variables|Default|GetcastedMagnetGameInstance) (Variables|Default|GetteamIndex) (Variables|Default|GetaddScore))
                  (bind _asattract_object_ball (Utilities|Casting|CastToAttractObject_Ball (Class|MagnetComponent|GetAttractActor (Variables|/Game/ThirdPersonBP/Blueprints/ThirdPersonCharacter.ThirdPersonCharacter_C|GetMagnet (Variables|Default|GetcastedPlayerActor))))
                    (:then
                      (Variables|Default|SetcastedAttractObject _asattract_object_ball))
                    (:CastFailed
                      (bind _asattract_object_ball_2 (Utilities|Casting|CastToAttractObject_Ball (Variables|Default|GethitActor)))
                      (Variables|Default|SetcastedAttractObject _asattract_object_ball_2)))
                  (Default|Goal (Variables|Default|GetcastedAttractObject) self)
                  (Class|MagnetComponent|DisableAttractObject (Variables|/Game/ThirdPersonBP/Blueprints/ThirdPersonCharacter.ThirdPersonCharacter_C|GetMagnet (Variables|Default|GetcastedPlayerActor)))))))))
      (else
        (Variables|Default|SetisPlayer false)
        (bind _array_element (Utilities|Array|ForEachLoopwithBreak (Variables|/Game/Blueprints/MagnetGameInstance.MagnetGameInstance_C|GetPlayerActorArray (Variables|Default|GetcastedMagnetGameInstance)) :!label _label_3)
          (:LoopBody
            (if (== _array_element (Variables|Default|GethitActor))
              (Variables|Default|SetisPlayer true)
              (goto _label_3 Break)))
          (:Completed
            (if (Variables|Default|GetisPlayer)
              (bind _asthird_person_character_2 (Utilities|Casting|CastToThirdPersonCharacter (Variables|Default|GethitActor)))
              (bind _output_get_3 (Variables|Default|SetcastedPlayerActor _asthird_person_character_2))
              (if (and (Class|MagnetComponent|IsAttractObjectIsBallActor (Variables|/Game/ThirdPersonBP/Blueprints/ThirdPersonCharacter.ThirdPersonCharacter_C|GetMagnet (Variables|Default|GetcastedPlayerActor))) (Utilities|IsValid _output_get_3))
                (Variables|Default|SetaddScore (Variables|Default|GetaddScoreTouchDown))
                (goto _label_2))
              (elif (== (Utilities|GetClass (Variables|Default|GethitActor)) "/Game/TEST/AttractTemp/AttractObject_Ball.AttractObject_Ball_C")
                (bind _asattract_object_ball_3 (Utilities|Casting|CastToAttractObject_Ball (Variables|Default|GethitActor))
                  (:then
                    (bind _asthird_person_character_3 (Utilities|Casting|CastToThirdPersonCharacter (Class|ItemShootComponent|GetWhoHave (Variables|/Game/TEST/AttractTemp/AttractObject.AttractObject_C|GetItemShoot _asattract_object_ball_3)))
                      (:then
                        (Variables|Default|SetcastedPlayerActor _asthird_person_character_3)
                        (if (Variables|/Script/Teleport.ItemShootComponent|Getm_IsShoot (Variables|/Game/TEST/AttractTemp/AttractObject.AttractObject_C|GetItemShoot _asattract_object_ball_3))
                          (Variables|Default|SetaddScore (Variables|Default|GetaddScoreShoot))
                          (goto _label_2)
                          (else
                            (Development|PrintString "Not Shoot"))))
                      (:CastFailed
                        (Development|PrintString (Utilities|String|BuildString(Object) "" "fail cast player : " (Class|ItemShootComponent|GetWhoHave (Variables|/Game/TEST/AttractTemp/AttractObject.AttractObject_C|GetItemShoot _asattract_object_ball_3)))))))
                  (:CastFailed
                    (Development|PrintString "fail cast ball")))
                (else
                  (Development|PrintString "not ball"))))))))))

(event EventTick
  (params (DeltaSeconds :type Float%20%28single-precision%29))
  (bind _arrow (Variables|Default|GetArrow))
  (if (Variables|Default|GetisGoal)
    (bind _output_get (Variables|Default|Settimer (+ DeltaSeconds (Variables|Default|Gettimer))))
    (if (> _output_get (Variables|Default|GetShootTime))
      (Variables|Default|SetisGoal false)
      (Variables|/Game/TEST/AttractTemp/AttractObject_Ball.AttractObject_Ball_C|SetisGoal (Variables|Default|GetcastedAttractObject) false)
      (CallFunction|SetArrowRandomRotation)
      (Variables|Default|SetShootPower (Math|Random|RandomFloatinRange (Variables|Default|GetShootPowerMin) (Variables|Default|GetShootPowerMax)))
      (Physics|AddImpulse (Variables|/Game/TEST/AttractTemp/AttractObject.AttractObject_C|GetBaseStaticMesh (Variables|Default|GetcastedAttractObject)) (* (CallFunction|GetArrowVector) (Variables|Default|GetShootPower)) "None" false)
      (Rendering|SetVisibility _arrow false false)
      (Variables|/Script/Engine.ArrowComponent|SetArrowLength _arrow (Math|Float|Lerp (Variables|デバッグ|GetArrowLengthMin) (Variables|デバッグ|GetArrowLengthMax) (/ (- (Variables|Default|GetShootPower) (Variables|Default|GetShootPowerMin)) (- (Variables|Default|GetShootPowerMax) (Variables|Default|GetShootPowerMin)))))
      (Rendering|SetVisibility _arrow true false))
    (else
      (Variables|Default|Settimer 0.0))))

(event EventBeginPlay
  (Variables|/Script/Engine.ArrowComponent|SetArrowLength (Variables|Default|GetArrow) (Variables|デバッグ|GetArrowLengthMin))
  (CallFunction|SetColor))

(fn ConstructionScript
  (CallFunction|SetColor))

(fn GetArrowVector
  (return (Math|Vector|GetForwardVector (Transformation|GetWorldRotation (Variables|Default|GetArrow)))))

(fn SetArrowRandomRotation
  (Transformation|SetRelativeRotation (Variables|Default|GetArrow) (Math|Rotator|MakeRotator 0.0 (Math|Random|RandomFloatinRange 0.0 (Variables|Default|GetShootDegreeMax)) (Math|Random|RandomFloatinRange (* -1 (Variables|Default|GetShootDegreeMax)) (Variables|Default|GetShootDegreeMax))) false false))

(fn SetColor
  (bind _color (Variables|Default|Getcolor))
  (Rendering|Material|SetDefaultCustomPrimitiveDataVector4 (Variables|Default|GetStaticMesh) 0 (Math|Vector4|MakeVector4 (.r _color) (.g _color) (.b _color) (.a _color))))