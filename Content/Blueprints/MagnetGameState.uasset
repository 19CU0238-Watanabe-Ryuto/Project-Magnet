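; Game state for a timed two-team match, handling the countdown, end-of-match sequence, player registry and team scores.
; BeginPlay shows the score UI, and an authority-only Tick advances the timer.
; At time-up it applies slow motion with a game-set widget, then restores speed, removes the minimap, switches to a tagged result camera and shows results.
; RunOnServer's additions to remaining time are overwritten by Tick's recalculation.
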(event Custom|RunOnServer
  (params (int :type Float%20%28single-precision%29))
  (Development|PrintString "Hello")
  (Variables|Default|SetremainTime (+ int (Variables|Default|GetremainTime))))

(event EventBeginPlay
  (bind _returnvalue (UserInterface|CreateWidget "/Game/UI/ScoreUI.ScoreUI_C"))
  (UserInterface|Viewport|AddtoViewport _returnvalue 0))

(event EventTick
  (params (DeltaSeconds :type Float%20%28single-precision%29))
  (bind _gametime (Variables|Default|GetGameTime))
  (bind _minimap (Variables|Default|GetminiMap))
  (Networking|SwitchHasAuthority
    (:Authority
      (bind _output_get (Variables|Default|SetTimer (+ DeltaSeconds (Variables|Default|GetTimer))))
      (Variables|Default|SetremainTime (- _gametime (Variables|Default|GetTimer)))
      (if (> _output_get _gametime)
        (Variables|Default|SetisGameSet true)
        (Variables|Default|SetremainTime 0.0)
        (Utilities|Time|SetGlobalTimeDilation (Variables|Default|GetSlowRatio))
        (if (> (- (Variables|Default|GetTimer) (Variables|Default|GetGameTime)) (* (Variables|Default|GetToResultTime) (Variables|Default|GetSlowRatio)))
          (Utilities|FlowControl|DoOnce false
            (:Completed
              (Widget|RemovefromParent (Variables|Default|GetGameSetUI))
              (Utilities|Time|SetGlobalTimeDilation 1.0)
              (Utilities|IsValid _minimap
                (:Is%20Valid
                  (Default|DeleteUI _minimap))
                (:Is%20Not%20Valid
                  _))
              (bind _outactors (Actor|GetAllActorsOfClasswithTag "/Script/Engine.CameraActor" "ResultCamera"))
              (Utilities|IsValid (Utilities|Array|Get(acopy) _outactors)
                (:Is%20Valid
                  (Game|Player|SetViewTargetwithBlend (Game|GetPlayerController 0) (Utilities|Array|Get(acopy) _outactors) 0.0 "VTBlend_Linear" 0.0 false))
                (:Is%20Not%20Valid
                  _))
              (bind _returnvalue (UserInterface|CreateWidget "/Game/UI/ResultUI.ResultUI_C"))
              (UserInterface|Viewport|AddtoViewport _returnvalue 0)))
          (else
            (Utilities|FlowControl|DoOnce false
              (:Completed
                (bind _returnvalue_2 (UserInterface|CreateWidget "/Game/UI/GameSetUI.GameSetUI_C"))
                (bind _output_get_2 (Variables|Default|SetGameSetUI _returnvalue_2))
                (UserInterface|Viewport|AddtoViewport _output_get_2 0)))))))))

(fn ConstructionScript)

(fn AddPlayer
  (params (_player :type Actor%20Object%20Reference))
  (bind _returnvalue (Utilities|Array|Add (Variables|Default|GetPlayerActorArray) _player))
  (Utilities|Casting|CastToThirdPersonCharacter _player)
  (return _returnvalue))

(fn SetScore
  (params (TeamIndex :type Integer) (Score :type Integer))
  (switch int TeamIndex
    (:0
      (Variables|Default|SetTeamScoreA (+ (Variables|Default|GetTeamScoreA) Score)))
    (:1
      (Variables|Default|SetTeamScoreB (+ (Variables|Default|GetTeamScoreB) Score)))))

(fn GetPlayerControllerIndexfromActor)