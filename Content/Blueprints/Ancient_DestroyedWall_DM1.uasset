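; Destructible ancient wall that breaks itself on a timer after play begins, then fades out and is destroyed.
; Once the break time elapses, Tick alternates through a FlipFlop between setting a no-pawn collision profile and applying bounds-scaled radius damage until a fracture event fires.
; After a further delay, it swaps to a translucent material and drives opacity down through custom primitive data before destroying the actor.
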(event Custom|PRINT
  (params (HitPoint :type Vector%20%28by%20ref%29) (HitDirection :type Vector%20%28by%20ref%29))
  (Variables|Default|SetisBroke true))

(event EventTick
  (params (DeltaSeconds :type Float%20%28single-precision%29))
  (Variables|Default|SetDelta%20Seconds DeltaSeconds)
  (if (Variables|Default|GetisBroke)
    (bind _output_get (Variables|Default|SetMaterialSwitchTimer (+ (Variables|Default|GetMaterialSwitchTimer) (Variables|Default|GetDelta%20Seconds))))
    (if (> _output_get (Variables|Default|GetMaterialSwitchTime))
      (Rendering|Material|SetMaterial (Variables|Default|GetDestructible) 0 "/Game/Geometry/AncientStage/DestroyedWall/Ancient_DestroyedWall_Translucent.Ancient_DestroyedWall_Translucent")
      (Utilities|Opacity (Variables|Default|GetDelta%20Seconds)))
    (else
      (Utilities|BeforeBreak (Variables|Default|GetDelta%20Seconds)))))

(event EventBeginPlay
  (EventDispatchers|BindEventtoOnComponentFracture (Variables|Default|GetDestructible) (delegate Custom|PRINT))
  (Variables|/Script/ApexDestruction.DestructibleComponent|SetLargeChunkThreshold (Variables|Default|GetDestructible) 5e+03))

(fn ConstructionScript)