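; Procedural road track actor that lays a chosen mesh along an editable spline.
; The construction script divides the spline length by the Divisor spacing and adds a collision-enabled spline mesh component for each interval.
; Each segment takes its start and end from local-space spline locations, with tangents formed by adding a Tangent offset to the spline direction.
; The event graph holds no active logic.
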(event EventBeginPlay)

(event Collision|EventActorBeginOverlap
  (params (OtherActor :type Actor%20Object%20Reference)))

(event EventTick
  (params (DeltaSeconds :type Float%20%28single-precision%29)))

(fn ConstructionScript
  (bind _divisor (Variables|Default|GetDivisor))
  (bind _spline (Variables|Default|GetSpline))
  (for _index (range 0 (.ReturnValue (Math|Float|Division(WholeandRemainder) (Spline|GetSplineLength (Variables|Default|GetSpline)) (Variables|Default|GetDivisor))))
    (Variables|Default|SetDistanceA (* _index _divisor))
    (Variables|Default|SetDistanceB (+ (* _index _divisor) _divisor))
    (bind _returnvalue (AddComponent|AddSplineMeshComponent false))
    (Components|StaticMesh|SetStaticMesh _returnvalue (Variables|Default|GetMesh))
    (Collision|SetCollisionEnabled _returnvalue "QueryAndPhysics")
    (SplineMesh|SetStartandEnd _returnvalue (Spline|GetLocationatDistanceAlongSpline _spline (Variables|Default|GetDistanceA) "Local") (+ (Spline|GetDirectionatDistanceAlongSpline _spline (Variables|Default|GetDistanceA) "Local") (Variables|Default|Gettangent)) (Spline|GetLocationatDistanceAlongSpline _spline (Variables|Default|GetDistanceB) "Local") (+ (Spline|GetDirectionatDistanceAlongSpline _spline (Variables|Default|GetDistanceB) "Local") (Variables|Default|Gettangent)) true :!class /Script/Engine.SplineMeshComponent)))