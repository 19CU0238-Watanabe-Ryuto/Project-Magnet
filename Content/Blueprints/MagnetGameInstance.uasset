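; Game instance for the Magnet game that holds a player list and running scores for two teams.
; Init clears the player array, and AddPlayer appends a player and returns its index.
; SetScore adds the given amount to team A or B by team index, rather than overwriting the total.
; BeginGameHost is an empty event, and a session node with a LAN option sits unconnected, so it never runs.
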(event Custom|BeginGameHost)

(event EventInit
  (Utilities|Array|Clear (Variables|Default|GetPlayerActorArray)))

(fn AddPlayer
  (params (_player :type Actor%20Object%20Reference))
  (bind _returnvalue (Utilities|Array|Add (Variables|Default|GetPlayerActorArray) _player))
  (return _returnvalue))

(fn SetScore
  (params (TeamIndex :type Integer) (Score :type Integer))
  (switch int TeamIndex
    (:0
      (Variables|Default|SetTeamScoreA (+ (Variables|Default|GetTeamScoreA) Score)))
    (:1
      (Variables|Default|SetTeamScoreB (+ (Variables|Default|GetTeamScoreB) Score)))))