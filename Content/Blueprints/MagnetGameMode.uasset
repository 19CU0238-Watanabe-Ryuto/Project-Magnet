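; Game mode for a magnet game that spawns and possesses a character for each player on login.
; Join order picks the class from an array, falling back to ThirdPersonCharacter, selects the numbered PlayerStart, and alternates the pawn's MagnetType between two values.
; Each pawn's list index is stored in a map, which helper functions use to look up an actor's player controller or index, printing a message for unmanaged actors.
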(event EventPostLogin
  (params (NewPlayer :type Player%20Controller%20Object%20Reference))
  (bind _playerpawnlist (Variables|Default|GetPlayerPawnList))
  (bind _returnvalue (Utilities|Array|Length _playerpawnlist))
  (bind _returnvalue_2 (+ _returnvalue 1))
  (bind _returnvalue_3 (Utilities|String|BuildString(Integer) "" "Player" _returnvalue_2))
  (Development|PrintString (Utilities|String|Append _returnvalue_3 ":Login "))
  (Utilities|SwitchSpawnCharacter)
  (bind _returnvalue_4 (Game|SpawnActorfromClass (Variables|Default|GetSpawnCharacter) (Transformation|GetActorTransform (Class|GameModeBase|FindPlayerStart NewPlayer _returnvalue_3)) "Undefined" 0 0))
  (if (== (Math|Integer|%(Integer) (Utilities|Array|Length (Variables|Default|GetPlayerPawnList)) 2) 0)
    (Variables|/Game/ThirdPersonBP/Blueprints/ThirdPersonCharacter.ThirdPersonCharacter_C|SetMagnetType _returnvalue_4 "NewEnumerator0")
    (else
      (Variables|/Game/ThirdPersonBP/Blueprints/ThirdPersonCharacter.ThirdPersonCharacter_C|SetMagnetType _returnvalue_4 "NewEnumerator1")))
  (bind _returnvalue_5 (Utilities|Array|Add (Variables|Default|GetPlayerPawnList) _returnvalue_4))
  (Utilities|Map|Add (Variables|Default|GetPlayerControllerIDMap) _returnvalue_4 _returnvalue_5)
  (Pawn|Possess NewPlayer _returnvalue_4))

(fn ConstructionScript)

(fn GetPlayerControllerIndexfromActor
  (params (TargetActor :type Actor%20Object%20Reference))
  (bind _playercontrolleridmap (Variables|Default|GetPlayerControllerIDMap))
  (bind (_value _returnvalue) (Utilities|Map|Find _playercontrolleridmap TargetActor))
  (if _returnvalue
    (return _value)
    (else
      (Development|PrintString (Utilities|String|Append (Utilities|GetDisplayName TargetActor) " : is not managed by GameMode")))))

(fn GetPlayerControllerfromActor
  (params (TargetActor :type Actor%20Object%20Reference))
  (bind _playercontrolleridmap (Variables|Default|GetPlayerControllerIDMap))
  (bind (_value _returnvalue) (Utilities|Map|Find _playercontrolleridmap TargetActor))
  (if _returnvalue
    (return (Game|GetPlayerController _value))
    (else
      (Development|PrintString (Utilities|String|Append (Utilities|GetDisplayName TargetActor) " : is not managed by GameMode")))))